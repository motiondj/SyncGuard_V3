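; Demo actor for testing nDisplay JSON cluster events from the keyboard, with input enabled only on the instance flagged IsPrimary.
; Number keys emit single, multiple or same-name events as primary-only, or from any node with Left Shift held.
; Received events print their contents plus a Tick-driven frame counter to check same-frame arrival.
; Add and Subtract keys spawn or destroy extra copies of the actor as listeners.
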(event EventBeginPlay
  ;[1 1 1] Enable input to be able to generate cluster events from keyboard.
  ; NOTE: Make sure you set bIsPrimary flag to enable input for the BP instance.
  (if (Variables|Default|GetbIsPrimary)
    (Input|EnableInput (Game|GetPlayerController 0))))

(event EventOnClusterEventJson
  (params (Event :type Display%20Cluster%20Cluster%20Event%20Json%20Structure%20%28by%20ref%29))
  (bind (_name _type _category _parameters) (Utilities|Struct|BreakDisplayClusterClusterEventJson Event))
  ;[1 1 1] Process cluster event (print event's data to the screen)
  (Development|PrintString (Utilities|String|Append "EVENT RECEIVED [ " (Utilities|String|ToString(Integer) (Variables|Default|GetFrameCount)) " ]"))
  (Variables|Default|SetLogMsg "")
  (bind _output_get (Variables|Default|SetEventParams _parameters))
  (if (> (Utilities|Map|Length _output_get) 0)
    (for _index (range 0 (- (Utilities|Map|Length _output_get) 1))
      (bind _keys (Utilities|Map|Keys (Variables|Default|GetEventParams)))
      (bind _values (Utilities|Map|Values (Variables|Default|GetEventParams)))
      (Variables|Default|SetLogMsg (Utilities|String|Append (Variables|Default|GetLogMsg) (Utilities|Array|Get(acopy) _keys _index) "=" (Utilities|Array|Get(acopy) _values _index) "; "))))
  (Development|PrintString (Utilities|String|Append "EVENT: " _category " : " _type " : " _name "   :->: " (Variables|Default|GetLogMsg))))

(event EventTick
  (params (DeltaSeconds :type Float%20%28single-precision%29))
  ;[1 1 1] Increment the frame counter to make sure all events come on the same frame
  (Math|Integer|IncrementInt (Variables|Default|GetFrameCount)))

(event Input|KeyboardEvents|2
  (params (Key :type Key%20Structure :default "None"))
  (bind _returnvalue (Game|GetPlayerController 0))
  (bind _returnvalue_2 (Game|Player|IsInputKeyDown _returnvalue "LeftShift"))
  (bind _returnvalue_3 (not _returnvalue_2))
  (bind _returnvalue_4 (select _returnvalue_3 "TEST_MULT_PRIMARY" "TEST_MULT_NODE"))
  ;[1 1 1] TEST: Emit two cluster events from master PC only (unique events). If left shift is pressed, emits from any cluster node.
  (:Pressed
    (Development|PrintString "TEST 2")
    (Class|DisplayClusterBlueprintLib|EmitClusterEventJson (Utilities|Struct|MakeDisplayClusterClusterEventJson "TEST_EVENT_1" _returnvalue_4 "TEST" (Utilities|Map|MakeMap "Key_0" "Val_0")) _returnvalue_3)
    (Class|DisplayClusterBlueprintLib|EmitClusterEventJson (Utilities|Struct|MakeDisplayClusterClusterEventJson "" _returnvalue_4 "" (Utilities|Map|MakeMap "Key_0" "Val_0" "Key_1" "Val_1")) _returnvalue_3)))

(event Input|KeyboardEvents|Add
  (params (Key :type Key%20Structure :default "None"))
  ;[1 1 1] Add one more listener
  (:Pressed
    (if (Variables|Default|GetbIsPrimary)
      (Development|PrintString "+1 Listener")
      (bind _returnvalue (Game|SpawnActorfromClass "BP_DemoClusterEvents_C" (Math|Transform|MakeTransform "0, 0, 0") "AlwaysSpawn" "OverrideRootScale" 0 0))
      (Utilities|Array|Add (Variables|Default|GetActorInstances) _returnvalue))))

(event Input|KeyboardEvents|3
  (params (Key :type Key%20Structure :default "None"))
  (bind _returnvalue (Game|GetPlayerController 0))
  (bind _returnvalue_2 (Game|Player|IsInputKeyDown _returnvalue "LeftShift"))
  (bind _returnvalue_3 (not _returnvalue_2))
  (bind _returnvalue_4 (select _returnvalue_3 "TEST_MULT_PRIMARY" "TEST_MULT_NODE"))
  ;[1 1 1] TEST: Emit three cluster events from master PC only (unique events). If left shift is pressed, emits from any cluster node.
  (:Pressed
    (Development|PrintString "TEST 3")
    (Class|DisplayClusterBlueprintLib|EmitClusterEventJson (Utilities|Struct|MakeDisplayClusterClusterEventJson "TEST_EVENT_1" _returnvalue_4 "TEST" (Utilities|Map|MakeMap "Key_0" "Val_0")) _returnvalue_3)
    (Class|DisplayClusterBlueprintLib|EmitClusterEventJson (Utilities|Struct|MakeDisplayClusterClusterEventJson "TEST_EVENT_2" _returnvalue_4 "TEST" (Utilities|Map|MakeMap)) _returnvalue_3)
    (Class|DisplayClusterBlueprintLib|EmitClusterEventJson (Utilities|Struct|MakeDisplayClusterClusterEventJson "TEST_EVENT_3" _returnvalue_4 "TEST" (Utilities|Map|MakeMap "Key_0" "Val_0" "Key_1" "Val_1" "Key_2" "Val_2")) _returnvalue_3)))

(event Input|KeyboardEvents|1
  (params (Key :type Key%20Structure :default "None"))
  (bind _returnvalue (Game|GetPlayerController 0))
  (bind _returnvalue_2 (Game|Player|IsInputKeyDown _returnvalue "LeftShift"))
  (bind _returnvalue_3 (not _returnvalue_2))
  ;[1 1 1] TEST: Emit single cluster event from master PC only. If left shift is pressed, emits from any cluster node.
  (:Pressed
    (Development|PrintString "TEST 1")
    (Class|DisplayClusterBlueprintLib|EmitClusterEventJson (Utilities|Struct|MakeDisplayClusterClusterEventJson "TEST_EVENT" (select _returnvalue_3 "TEST_SINGLE_PRIMARY" "TEST_SINGLE_NODE") "TEST" (Utilities|Map|MakeMap "Key_0" "Val_0" "Key_1" "Val_1")) _returnvalue_3)))

(event Input|KeyboardEvents|Subtract
  (params (Key :type Key%20Structure :default "None"))
  (bind _actorinstances (Variables|Default|GetActorInstances))
  (bind _returnvalue (Utilities|Array|Length _actorinstances))
  ;[1 1 1] Remove one listener
  (:Pressed
    (if (Variables|Default|GetbIsPrimary)
      (if (> _returnvalue 0)
        (Actor|DestroyActor (Utilities|Array|Get(acopy) (Variables|Default|GetActorInstances)))
        (Utilities|Array|RemoveIndex (Variables|Default|GetActorInstances))
        (Development|PrintString (Utilities|String|Append "-1 Listener, left: " (Utilities|String|ToString(Integer) _returnvalue)))))))

(event Input|KeyboardEvents|4
  (params (Key :type Key%20Structure :default "None"))
  (bind _returnvalue (Game|GetPlayerController 0))
  (bind _returnvalue_2 (Game|Player|IsInputKeyDown _returnvalue "LeftShift"))
  (bind _returnvalue_3 (not _returnvalue_2))
  (bind _returnvalue_4 (select _returnvalue_3 "TEST_MULT_PRIMARY" "TEST_MULT_NODE"))
  ;[1 1 1] TEST: Emit two cluster events from master node (duplicated events). If left shift is pressed, emits from any cluster node.
  (:Pressed
    (Development|PrintString "TEST 2")
    (Class|DisplayClusterBlueprintLib|EmitClusterEventJson (Utilities|Struct|MakeDisplayClusterClusterEventJson "TEST_EVENT_DUPL" _returnvalue_4 "TEST" (Utilities|Map|MakeMap "Key_0" "Val_0")) _returnvalue_3)
    (Class|DisplayClusterBlueprintLib|EmitClusterEventJson (Utilities|Struct|MakeDisplayClusterClusterEventJson "TEST_EVENT_DUPL" _returnvalue_4 "TEST" (Utilities|Map|MakeMap "Key_0" "Val_0" "Key_1" "Val_1")) _returnvalue_3)
    (Class|DisplayClusterBlueprintLib|EmitClusterEventJson (Utilities|Struct|MakeDisplayClusterClusterEventJson "TEST_EVENT_DUPL" _returnvalue_4 "TEST" (Utilities|Map|MakeMap "Key_0_LAST" "Val_0_LAST" "Key_1_LAST" "Val_1_LAST")) _returnvalue_3)))

(fn ConstructionScript)